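; Test player Character with Enhanced Input movement, mouse-style look and a custom multi-jump.
; BeginPlay adds the IMC_Play mapping context and resets jump state; move inputs follow control yaw.
; Jump input uses LaunchCharacter with separate ground and air Z velocities up to JumpCountMax, and OnLanded resets the count.
; Tick and jump events print debug state; legacy axis events and older jump and movement logic remain disconnected.
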(event `Player_Init`
  ;[1 1 1] プレイヤーの状態初期化
  (set `self.Is_Jumping` false)
  (set `self.Jump_Count` 0)
  (set `self.Jump_CountMax` (`self.Jump_CountMax`)))

(event `self.ReceiveBeginPlay`
  (`|ExecutionSequence`
    (:`then_0`
      (`self.ControllerMapping`) ; プレイヤーの入力操作割り当て
      (`self.Player_Init`))))

(event `self.ReceiveTick`
  (params (DeltaSeconds :type "Float (single-precision)"))
  (`self.Debug_PlayerState`))

(event `InputAxis|Look Up / Down Mouse`
  (params (AxisValue :type "Float (single-precision)"))
  ;[0 0 0] プレイヤーの視点移動(UE4)
)

(event `Debug_PlayerState`
  ;[1 1 1] デバッグ：プレイヤーの状況確認
  (`|ExecutionSequence`
    (:`then_0`
      (if true
        (`KismetSystemLibrary.PrintString` "Ready:Jump" true true (struct :`G` 1.0 :`A` 1.0) 0.0)))
    (:`then_1`
      (if (`self.Is_Jumping`)
        (`KismetSystemLibrary.PrintString` "State:Air" true true (struct :`G` 1.0 :`A` 1.0) 0.0)
        (else
          (`KismetSystemLibrary.PrintString` "State:Ground" true true (struct :`G` 1.0 :`A` 1.0) 0.0))))))

(event `ControllerMapping`
  (bind _returnvalue (`GameplayStatics.GetPlayerController` 0))
  ;[1 1 1] プレイヤーのインプットマッピングシステム（入力操作割り当て）
  (`/Engine/EditorBlueprintResources/StandardMacros.IsValid` _returnvalue ; 有効であるか確認
    (:`Is Valid`
      (`EnhancedInputSubsystemInterface.AddMappingContext` (pcsubsystem `EnhancedInputLocalPlayerSubsystem` _returnvalue) "/Game/_MyContent/Input/IMC_Play.IMC_Play" 0 (struct)) ; Enhancedシステムを使って、操作キーバインドの\n設定を行う。
    )
    (:`Is Not Valid`
      (`KismetSystemLibrary.PrintString` "Error:PlayerContllo"))))

(event `InputAxis|Turn Right / Left Mouse`
  (params (AxisValue :type "Float (single-precision)"))
  ;[0 0 0] プレイヤーの視点移動(UE4)
)

(event `EnhancedInput|/Game/_MyContent/Input/IA_Jump_T`
  (params (ActionValue :type Boolean) (ElapsedSeconds :type "Float (double-precision)") (TriggeredSeconds :type "Float (double-precision)") (InputAction :type "InputAction Object Reference" :default "/Game/_MyContent/Input/IA_Jump_T.IA_Jump_T"))
  ;[1 1 1] プレイヤーのジャンプ処理
  (:`Started`
    (if (< (`self.Jump_Count`) (`self.Jump_CountMax`))
      (if (`NavMovementComponent.IsFalling` (`self.CharacterMovement`))
        ;;[1 1 1] 空中ジャンプの処理
        (`self.LaunchCharacter` (`KismetMathLibrary.MakeVector` 0.0 0.0 (`self.Jump_AirVelocity`)) false true) ; プレイヤーへZ軸方向の力を加える
        (set `self.Jump_Count` (+ (`self.Jump_Count`) 1)) ; ジャンプ回数をカウント
        (`KismetSystemLibrary.PrintString` "Air_Jump")
        (else
          ;;[1 1 1] 地上ジャンプの処理
          (`self.LaunchCharacter` (`KismetMathLibrary.MakeVector` 0.0 0.0 (`self.Jump_GroundVelocity`)) false true) ; プレイヤーへZ軸方向の力を加える
          (set `self.Is_Jumping` true) ; 空中にいる判定に変更
          (set `self.Jump_Count` (+ (`self.Jump_Count`) 1)) ; ジャンプ回数をカウント
          (`KismetSystemLibrary.PrintString` "Ground_Jump")))
      (else
        (`KismetSystemLibrary.PrintString` "Can't Jump")))))

(event `InputAxis|Move Forward / Backward`
  (params (AxisValue :type "Float (single-precision)"))
  ;[0 0 0] プレイヤーの基本移動(UE4)
)

(event `EnhancedInput|/Game/_MyContent/Input/IA_Move_Forward`
  (params (ActionValue :type "Float (double-precision)") (ElapsedSeconds :type "Float (double-precision)") (TriggeredSeconds :type "Float (double-precision)") (InputAction :type "InputAction Object Reference" :default "/Game/_MyContent/Input/IA_Move_Forward.IA_Move_Forward"))
  ;[1 1 1] プレイヤーの基本移動
  (:`Triggered`
    (`self.AddMovementInput` (`KismetMathLibrary.GetForwardVector` (`KismetMathLibrary.MakeRotator` 0.0 0.0 (.yaw (`self.GetControlRotation`)))) ActionValue)))

(event `self.OnLanded`
  (params (Hit :type "HitResult Structure (by ref)"))
  ;[1 1 1] プレイヤーのジャンプ処理
  ;;[1 1 1] 着地処理
  (`self.StopJumping`)
  (set `self.Is_Jumping` false) ; ジャンプ中を解除
  (set `self.Jump_Count` 0)
  (`KismetSystemLibrary.PrintString` "Landing"))

(event `InputAxis|Move Right / Left`
  (params (AxisValue :type "Float (single-precision)"))
  ;[0 0 0] プレイヤーの基本移動(UE4)
)

(event `EnhancedInput|/Game/_MyContent/Input/IA_Move_Right`
  (params (ActionValue :type "Float (double-precision)") (ElapsedSeconds :type "Float (double-precision)") (TriggeredSeconds :type "Float (double-precision)") (InputAction :type "InputAction Object Reference" :default "/Game/_MyContent/Input/IA_Move_Right.IA_Move_Right"))
  ;[1 1 1] プレイヤーの基本移動
  (:`Triggered`
    (`self.AddMovementInput` (`KismetMathLibrary.GetRightVector` (`KismetMathLibrary.MakeRotator` 0.0 0.0 (.yaw (`self.GetControlRotation`)))) ActionValue)))

(event `EnhancedInput|/Game/_MyContent/Input/IA_Jump_T`
  (params (ActionValue :type Boolean) (ElapsedSeconds :type "Float (double-precision)") (TriggeredSeconds :type "Float (double-precision)") (InputAction :type "InputAction Object Reference" :default "/Game/_MyContent/Input/IA_Jump_T.IA_Jump_T"))
  ;[0 0 0] UEの物理エンジンを用いたジャンプ機能
)

(event `EnhancedInput|/Game/_MyContent/Input/IA_Look_Up`
  (params (ActionValue :type "Float (double-precision)") (ElapsedSeconds :type "Float (double-precision)") (TriggeredSeconds :type "Float (double-precision)") (InputAction :type "InputAction Object Reference" :default "/Game/_MyContent/Input/IA_Look_Up.IA_Look_Up"))
  ;[1 1 1] プレイヤーの視点移動
  (:`Triggered`
    (`self.AddControllerPitchInput` ActionValue) ; 縦回転に値を適用する。
  ))

(event `CustomEvent`
  (params (MyComp :type "PrimitiveComponent Object Reference") (Other :type "Actor Object Reference") (OtherComp :type "PrimitiveComponent Object Reference") (bSelfMoved :type Boolean) (HitLocation :type "Vector Structure") (HitNormal :type "Vector Structure") (NormalImpulse :type "Vector Structure") (Hit :type "HitResult Structure (by ref)"))
  ;[0 0 0] UEの物理エンジンを用いたジャンプ機能
)

(event `EnhancedInput|/Game/_MyContent/Input/IA_Look_Right`
  (params (ActionValue :type "Float (double-precision)") (ElapsedSeconds :type "Float (double-precision)") (TriggeredSeconds :type "Float (double-precision)") (InputAction :type "InputAction Object Reference" :default "/Game/_MyContent/Input/IA_Look_Right.IA_Look_Right"))
  ;[1 1 1] プレイヤーの視点移動
  (:`Triggered`
    (`self.AddControllerYawInput` ActionValue) ; 水平方向の回転に値を適用する。
  ))

(fn `UserConstructionScript`)